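; Platformer game mode that persists the player's death count between sessions through a save game slot.
; On BeginPlay it waits a tick, caches the BP_TopDownCharacter_Platformer player character and restores its Deaths from BP_SaveGame, if a save exists.
; The SaveDeaths event writes the character's current Deaths to that slot, creating the save object when none exists.
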(event `self.ReceiveBeginPlay`
  (`KismetSystemLibrary.DelayUntilNextTick`)
  (bind _asbp_top_down_character_platformer (cast `/Game/Maps/Platformer/Platformer_Blueprints/Character/BP_TopDownCharacter_Platformer` (`GameplayStatics.GetPlayerCharacter` 0)))
  (set `self.Player BP` _asbp_top_down_character_platformer)
  (`self.LoadGame`))

(event `Save Deaths`
  (bind _returnvalue (`GameplayStatics.DoesSaveGameExist` "slot1"))
  (if _returnvalue
    (bind _returnvalue_2 (`GameplayStatics.LoadGameFromSlot` "slot1"))
    (bind _asbp_save_game (cast `/Game/Maps/Platformer/Platformer_Blueprints/BP_SaveGame` _returnvalue_2))
    (set `/Game/Maps/Platformer/Platformer_Blueprints/BP_SaveGame.StoredDeaths` (`/Game/Maps/Platformer/Platformer_Blueprints/Character/BP_TopDownCharacter_Platformer.Deaths` (`self.Player BP`)) _asbp_save_game)
    (`GameplayStatics.SaveGameToSlot` _returnvalue_2 "slot1")
    (else
      (bind _returnvalue_3 (`GameplayStatics.CreateSaveGameObject` "/Game/Maps/Platformer/Platformer_Blueprints/BP_SaveGame.BP_SaveGame_C"))
      (set `/Game/Maps/Platformer/Platformer_Blueprints/BP_SaveGame.StoredDeaths` (`/Game/Maps/Platformer/Platformer_Blueprints/Character/BP_TopDownCharacter_Platformer.Deaths` (`self.Player BP`)) _asbp_save_game)
      (`GameplayStatics.SaveGameToSlot` _returnvalue_3 "slot1"))))

(event `LoadGame`
  (bind _returnvalue (`GameplayStatics.DoesSaveGameExist` "slot1"))
  (if _returnvalue
    (bind _returnvalue_2 (`GameplayStatics.LoadGameFromSlot` "slot1"))
    (bind _asbp_save_game (cast `/Game/Maps/Platformer/Platformer_Blueprints/BP_SaveGame` _returnvalue_2))
    (set `/Game/Maps/Platformer/Platformer_Blueprints/Character/BP_TopDownCharacter_Platformer.Deaths` (`/Game/Maps/Platformer/Platformer_Blueprints/BP_SaveGame.StoredDeaths` _asbp_save_game) (`self.Player BP`))))

(fn `UserConstructionScript`)