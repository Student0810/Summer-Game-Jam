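; BP_RunningCharacter is the player character for a running, beer-collecting minigame with a difficulty menu and timed HUD.
; BeginPlay adds the input mapping and shows difficulty selection; PlayerStartminiGame swaps in the HUD and sets its timer from difficulty flags.
; Tick repeatedly binds a round-counter reset to the game mode's SpawnCheckpoints dispatcher and enables BeginProperCounting when the beer total equals one.
; Enhanced Input drives movement relative to control rotation, and Death halts it immediately.
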(event `self.ReceiveBeginPlay`
  (bind _asplayer_controller (cast `PlayerController` (`self.GetController`)))
  (bind _returnvalue (pcsubsystem `EnhancedInputLocalPlayerSubsystem` _asplayer_controller))
  (`/Engine/EditorBlueprintResources/StandardMacros.IsValid` _returnvalue
    (:`Is Valid`
      (`EnhancedInputSubsystemInterface.AddMappingContext` _returnvalue "/Game/Maps/Run/Player/MAP_Running.MAP_Running" 0 (struct))
      (bind _returnvalue_2 (`|CreateWidget` "/Game/Maps/Run/Player/Difficulty_Selection.Difficulty_Selection_C"))
      (`UserWidget.AddToViewport` _returnvalue_2 0))))

(event `EnhancedInput|/Game/Maps/Run/Player/IA_Move`
  (params (ActionValue :type "Vector2D Structure") (ElapsedSeconds :type "Float (double-precision)") (TriggeredSeconds :type "Float (double-precision)") (InputAction :type "InputAction Object Reference" :default "/Game/Maps/Run/Player/IA_Move.IA_Move"))
  (bind (_returnvalue_roll _returnvalue_pitch _returnvalue_yaw) (`KismetMathLibrary.BreakRotator` (`self.GetControlRotation`)))
  (bind (_returnvalue_roll_2 _returnvalue_pitch_2 _returnvalue_yaw_2) (`KismetMathLibrary.BreakRotator` (`self.GetControlRotation`)))
  (:`Triggered`
    (`self.AddMovementInput` (`KismetMathLibrary.GetRightVector` (`KismetMathLibrary.MakeRotator` _returnvalue_roll 0.0 _returnvalue_yaw)) ActionValue_X)
    (`self.AddMovementInput` (`KismetMathLibrary.GetForwardVector` (`KismetMathLibrary.MakeRotator` _returnvalue_roll_2 0.0 _returnvalue_yaw_2)) ActionValue_Y)))

(event `Player Start miniGame`
  (bind _widget_ref (`self.Widget Ref`))
  (bind _widget_ref_2 (`self.Widget Ref`))
  (bind _widget_ref_3 (`self.Widget Ref`))
  (`WidgetLayoutLibrary.RemoveAllWidgets`)
  (bind _returnvalue (`|CreateWidget` "/Game/Maps/Run/Player/HUD.HUD_C"))
  (bind _output_get (set `self.Widget Ref` _returnvalue))
  (`UserWidget.AddToViewport` _output_get 0)
  (if (`self.Medium?`)
    (set `/Game/Maps/Run/Player/HUD.Minute_Count` 1 _widget_ref_2)
    (set `/Game/Maps/Run/Player/HUD.Second_Count` 0 _widget_ref_2)
    (elif (`self.Hard?`)
      (set `/Game/Maps/Run/Player/HUD.Minute_Count` 0 _widget_ref_3)
      (set `/Game/Maps/Run/Player/HUD.Second_Count` 30 _widget_ref_3)
      (elif (`self.For the beer?`)
        (set `/Game/Maps/Run/Player/HUD.Minute_Count` 0 _widget_ref)
        (set `/Game/Maps/Run/Player/HUD.Second_Count` 30 _widget_ref)))))

(event `Death`
  (`MovementComponent.StopMovementImmediately` (`self.CharacterMovement`)))

(event `self.ReceiveTick`
  (params (DeltaSeconds :type "Float (single-precision)"))
  (`|ExecutionSequence`
    (:`then_0`
      (bind _asrunning_game_mode (cast `/Game/Maps/Run/Player/RunningGameMode` (`GameplayStatics.GetGameMode`)))
      (add `/Game/Maps/Run/Player/RunningGameMode.SpawnCheckpoints` _asrunning_game_mode (delegate `Reset round count`)))
    (:`then_1`
      (if (== (`self.Beers collected total`) 1)
        (set `self.Begin Proper counting` true)))))

(event `Reset round count`
  (set `self.Beers Collected in the round` 0)
  (set `self.Ammount of beers spawned` 0))

(fn `UserConstructionScript`)