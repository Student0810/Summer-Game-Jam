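; BP_Beerpong is the player Blueprint for the Beer Pong map, letting the player aim and lob balls.
; Enhanced Input look adds horizontal yaw only, and the lob action spawns a BeerPongBall at the SpawnArrow's location and rotation.
; A ShotLanded flag gates each throw and is cleared after spawning, with no reset in this graph.
; BeginPlay creates the HUD widget and adds it to the viewport.
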(event `EnhancedInput|/Game/Maps/Beer_Pong/Player/IA_LOOK`
  (params (ActionValue :type "Vector2D Structure") (ElapsedSeconds :type "Float (double-precision)") (TriggeredSeconds :type "Float (double-precision)") (InputAction :type "InputAction Object Reference" :default "/Game/Maps/Beer_Pong/Player/IA_LOOK.IA_LOOK"))
  (:`Triggered`
    (`self.AddControllerYawInput` ActionValue_X)))

(event `EnhancedInput|/Game/Maps/Beer_Pong/Player/IA_Lob`
  (params (ActionValue :type Boolean) (ElapsedSeconds :type "Float (double-precision)") (TriggeredSeconds :type "Float (double-precision)") (InputAction :type "InputAction Object Reference" :default "/Game/Maps/Beer_Pong/Player/IA_Lob.IA_Lob"))
  (bind _spawn_arrow (`self.Spawn Arrow`))
  (:`Triggered`
    (if (`self.ShotLanded`)
      (`|SpawnActorFromClass` "/Game/Maps/Beer_Pong/Player/BeerPongBall.BeerPongBall_C" (`KismetMathLibrary.MakeTransform` (`SceneComponent.K2_GetComponentLocation` _spawn_arrow) (`SceneComponent.K2_GetComponentRotation` _spawn_arrow)) "AdjustIfPossibleButAlwaysSpawn" "MultiplyWithRoot" null null)
      (set `self.ShotLanded` false))))

(event `self.ReceiveBeginPlay`
  (bind _returnvalue (`|CreateWidget` "/Game/Maps/Beer_Pong/Player/HUD.HUD_C"))
  (`UserWidget.AddToViewport` _returnvalue 0))

(fn `UserConstructionScript`)